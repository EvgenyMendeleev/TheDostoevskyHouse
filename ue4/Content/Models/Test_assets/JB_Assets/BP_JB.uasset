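; BP_JB is a test Blueprint that drives animation state on its JB skeletal mesh through the ABP_JB Animation Blueprint.
; BeginPlay casts the mesh's anim instance to ABP_JB and caches it.
; Custom events then set that instance's Start and Switch booleans on or off, leaving the actual animation logic to the Animation Blueprint.
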(event Custom|St_BP
  (Variables|/Game/Models/Test_assets/JB_Assets/ABP_JB.ABP_JB_C|SetStart (stale EventBeginPlay _asabp_jb) true))

(event Custom|Bc_BP
  (Variables|/Game/Models/Test_assets/JB_Assets/ABP_JB.ABP_JB_C|SetStart (stale EventBeginPlay _asabp_jb) false))

(event Custom|SwCH_BP
  (Variables|/Game/Models/Test_assets/JB_Assets/ABP_JB.ABP_JB_C|SetSwitch (stale EventBeginPlay _asabp_jb) true))

(event Custom|SwCH_OFF_BP
  (Variables|/Game/Models/Test_assets/JB_Assets/ABP_JB.ABP_JB_C|SetSwitch (stale EventBeginPlay _asabp_jb) false))

(event EventBeginPlay
  (bind _asabp_jb (Utilities|Casting|CastToABP_JB (Components|SkeletalMesh|GetAnimInstance (Variables|Default|GetJB)))))

(fn ConstructionScript)