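; VR hand actor for the player that grabs and releases nearby objects.
; The construction script sets the motion source from the Hand enum and picks a glove mesh, assigning the right model to Left and vice versa.
; Grab finds the nearest GrabSphere overlap implementing the Grabable interface, stores it and sends GrabMessage with itself.
; Release sends ReleaseMessage to the held item and clears it, leaving attachment behavior to the item.
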(fn ConstructionScript
  (bind _hand (Variables|Default|GetHand))
  (bind _handmesh (Variables|Default|GetHandMesh))
  (Variables|/Script/HeadMountedDisplay.MotionControllerComponent|SetMotionSource (Variables|Default|GetVR_hand) (Utilities|Name|EnumtoName _hand))
  (switch Utilities|FlowControl|Switch|SwitchonEControllerHand _hand
    (:Left
      (Class|SkinnedMeshComponent|SetSkeletalMesh _handmesh "/Game/Models/vr_glove_right_model.vr_glove_right_model" true))
    (:Right
      (Class|SkinnedMeshComponent|SetSkeletalMesh _handmesh "/Game/Models/vr_glove_left_model.vr_glove_left_model" true))))

(fn TryGetNearActor
  (bind _grabsphere (Variables|Default|GetGrabSphere))
  (for _array_element (Collision|GetOverlappingActors _grabsphere 0 :!class /Script/Engine.PrimitiveComponent)
    (if (Utilities|DoesObjectImplementInterface _array_element "/Game/Blueprints/Interfaces/Grabable.Grabable_C")
      (if (< (Math|Vector|VectorLength (- (Transformation|GetActorLocation _array_element) (Transformation|GetWorldLocation _grabsphere))) (LocalVariables|GetNearestOverlap))
        (LocalVariables|SetNearestOverlappingActor _array_element)
        (LocalVariables|SetNearestOverlap (Math|Vector|VectorLength (- (Transformation|GetActorLocation _array_element) (Transformation|GetWorldLocation _grabsphere)))))))
  (return (LocalVariables|GetNearestOverlappingActor)))

(fn Grab
  (bind _nearestmesh (Interaction|TryGetNearActor))
  (Utilities|IsValid _nearestmesh
    (:Is%20Valid
      (bind _output_get (Variables|Default|SetGrabedItem _nearestmesh))
      (Class|Grabable|Grab(Message) _output_get self))))

(fn Release
  (Utilities|IsValid (Variables|Default|GetGrabedItem)
    (:Is%20Valid
      (Class|Grabable|Release(Message) (Variables|Default|GetGrabedItem))
      (Variables|Default|SetGrabedItem 0))))