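; CharacterVR is the player's VR character, with floor-level tracking, camera-relative movement and two grabbing hands.
; On BeginPlay it spawns left and right VR_Hand actors attached to the VR origin, and interact inputs drive their grab and release.
; Every tick, eight horizontal line traces from the HMD camera offset the character away from actors whose first tag is BlockCamera, keeping the head out of barriers.
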(event EventTick
  (params (DeltaSeconds :type Float%20%28single-precision%29))
  (CallFunction|CheckBarriersforHMD))

(event EventBeginPlay
  (bind _returnvalue (Math|Transform|MakeTransform "0, 0, 0" "0, 0, 0" "3.200000,3.200000,3.200000"))
  (bind _self self)
  (bind _vr_origin (Variables|Default|GetVR_Origin))
  (Class|HeadMountedDisplayFunctionLibrary|SetTrackingOrigin "Floor")
  ;[1 1 1] Hands Spawn
  (Utilities|FlowControl|Sequence
    (:then_0
      (bind _returnvalue_2 (Game|SpawnActorfromClass "/Game/Blueprints/Player/VR_Hand.VR_Hand_C" _returnvalue "Undefined" _self "Left" 0))
      (bind _output_get (Variables|Hands|SetLeftHand _returnvalue_2))
      (Transformation|AttachComponentToComponent _output_get _vr_origin "None" "SnapToTarget" "SnapToTarget" "KeepWorld" false))
    (:then_1
      (bind _returnvalue_3 (Game|SpawnActorfromClass "/Game/Blueprints/Player/VR_Hand.VR_Hand_C" _returnvalue "Undefined" _self "Right" 0))
      (bind _output_get_2 (Variables|Hands|SetRightHand _returnvalue_3))
      (Transformation|AttachComponentToComponent _output_get_2 _vr_origin "None" "SnapToTarget" "SnapToTarget" "KeepWorld" false))))

(event Input|ActionEvents|InputActionRightHandInteract
  (params (Key :type Key%20Structure :default "None"))
  (bind _righthand (Variables|Hands|GetRightHand))
  ;[1 1 1] Hands interaction
  (:Pressed
    (Default|Grab _righthand))
  (:Released
    (Default|Release _righthand)))

(event Input|ActionEvents|InputActionLeftHandInteract
  (params (Key :type Key%20Structure :default "None"))
  (bind _lefthand (Variables|Hands|GetLeftHand))
  ;[1 1 1] Hands interaction
  (:Pressed
    (Default|Grab _lefthand))
  (:Released
    (Default|Release _lefthand)))

(event Input|AxisEvents|InputAxisMoveForward
  (params (AxisValue :type Float%20%28single-precision%29))
  ;[1 1 1] Movement
  (CallFunction|Move AxisValue))

(event Input|AxisEvents|InputAxisMoveBack
  (params (AxisValue :type Float%20%28single-precision%29))
  ;[1 1 1] Movement
  (CallFunction|Move AxisValue))

(fn ConstructionScript)

(fn Move
  (params (Direction :type Float%20%28single-precision%29))
  (bind _camera (Variables|Default|GetCamera))
  (bind _returnvalue (Math|Vector|GetForwardVector _camera))
  (Pawn|Input|AddMovementInput (Math|Vector|MakeVector (.x _returnvalue) (.y _returnvalue) 0.0) (* (Variables|MovementSettings|GetMovementSpeed) Direction) false))

(fn CheckBarriersforHMD
  (for _array_element (Utilities|Array|MakeArray "1.000000, 0, 0" "0,1.000000, 0" "-1.000000,0.000000, 0" "0.000000,-1.000000, 0" "0.500000,0.500000, 0" "-0.500000,0.500000, 0" "0.500000,-0.500000, 0" "-0.500000,-0.500000, 0")
    (bind (_outhit _ishit) (CallFunction|Raycast (Transformation|GetWorldLocation (Variables|Default|GetCamera)) _array_element))
    (if _ishit
      (Development|PrintString (Utilities|String|ToString(Name) (Utilities|Array|Get(acopy) (Variables|/Script/Engine.Actor|GetTags (.HitActor (Collision|BreakHitResult _outhit))))))
      (if (Utilities|Name|Equal(Name) "BlockCamera" (Utilities|Array|Get(acopy) (Variables|/Script/Engine.Actor|GetTags (.HitActor (Collision|BreakHitResult _outhit)))))
        (Transformation|AddActorWorldOffset (Math|Vector|MakeVector (.x (* (Math|Vector|NegateVector _array_element) (Variables|BlockSettingsForHMD|GetTeleportDistance))) (.y (* (Math|Vector|NegateVector _array_element) (Variables|BlockSettingsForHMD|GetTeleportDistance))) 0.0) false true)))))

(fn Raycast
  (params (Start :type Vector) (Direction :type Vector))
  (bind (_outhit _returnvalue) (Collision|LineTraceByChannel Start (+ Start (* (/ Direction (Math|Vector|VectorLength Direction)) (Variables|BlockSettingsForHMD|GetLengthOfHMD_CheckLine))) "TraceTypeQuery1" false 0 "None"))
  (return _outhit _returnvalue))