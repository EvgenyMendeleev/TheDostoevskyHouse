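; VR player character that provides two motion-controller hands, walking and a toggleable main menu.
; BeginPlay sets floor tracking and spawns left and right BP_VR_Hand actors on VROrigin; interact inputs drive their grab and release.
; Axis inputs move along the camera's horizontal forward, SpawnQ spawns or destroys BP_MainMenu at the character, and Quit exits.
; Headset-driven camera, capsule and origin alignment functions exist but are disconnected, as Tick is empty.
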(event EventTick
  (params (DeltaSeconds :type Float%20%28single-precision%29))
  ;[1 1 1] CollisionAndNotViewAroundObject
)

(event EventBeginPlay
  (bind _returnvalue (Math|Transform|MakeTransform "0, 0, 0" "0, 0, 0" "3.200000,3.200000,3.200000"))
  (bind _self self)
  (bind _vrorigin (Variables|Default|GetVROrigin))
  ;[1 1 1] SpawnHandController
  (Class|HeadMountedDisplayFunctionLibrary|SetTrackingOrigin "Floor")
  (Utilities|FlowControl|Sequence
    (:then_0
      (bind _returnvalue_2 (Game|SpawnActorfromClass "/Game/Core/Player/BP_VR_Hand.BP_VR_Hand_C" _returnvalue "Undefined" _self "Left" 0))
      (bind _output_get (Variables|Hand|SetLeftHand _returnvalue_2))
      (Transformation|AttachComponentToComponent _output_get _vrorigin "None" "SnapToTarget" "SnapToTarget" "KeepWorld" false))
    (:then_1
      (bind _returnvalue_3 (Game|SpawnActorfromClass "/Game/Core/Player/BP_VR_Hand.BP_VR_Hand_C" _returnvalue "Undefined" _self "Right" 0))
      (bind _output_get_2 (Variables|Hand|SetRightHand _returnvalue_3))
      (Transformation|AttachComponentToComponent _output_get_2 _vrorigin "None" "SnapToTarget" "SnapToTarget" "KeepWorld" false))))

(event Input|ActionEvents|InputActionLeftHandInteract
  (params (Key :type Key%20Structure :default "None"))
  (bind _lefthand (Variables|Hand|GetLeftHand))
  ;[1 1 1] Hands interaction
  (:Pressed
    (Default|Grab _lefthand))
  (:Released
    (Default|Release _lefthand)))

(event Input|ActionEvents|InputActionQuit
  (params (Key :type Key%20Structure :default "None"))
  ;[1 1 1] Quit
  (:Pressed
    (Game|QuitGame 0 "Quit" false)))

(event Input|ActionEvents|InputActionSpawnQ
  (params (Key :type Key%20Structure :default "None"))
  (:Pressed
    (if (Math|Boolean|Equal(Boolean) (Variables|Default|GetReSpawn) false)
      (Actor|DestroyActor (stale _returnvalue))
      (Variables|Default|SetReSpawn true)
      (else
        (bind _returnvalue (Game|SpawnActorfromClass "/Game/GUI/BP_MainMenu.BP_MainMenu_C" (Transformation|GetActorTransform) "Undefined" 0 0))
        (Variables|Default|SetReSpawn false)))))

(event Input|ActionEvents|InputActionPause
  (params (Key :type Key%20Structure :default "None")))

(event Input|ActionEvents|InputActionRightHandInteract
  (params (Key :type Key%20Structure :default "None"))
  (bind _righthand (Variables|Hand|GetRightHand))
  ;[1 1 1] Hands interaction
  (:Pressed
    (Default|Grab _righthand))
  (:Released
    (Default|Release _righthand)))

(event Input|ActionEvents|InputActionRightHandInteract
  (params (Key :type Key%20Structure :default "None"))
  ;[0.1468 1 0] GUI Interaction
)

(event Input|AxisEvents|InputAxisMoveForward
  (params (AxisValue :type Float%20%28single-precision%29))
  ;[1 1 1] Movement
  (CallFunction|Move AxisValue))

(event Input|AxisEvents|InputAxisMoveBack
  (params (AxisValue :type Float%20%28single-precision%29))
  ;[1 1 1] Movement
  (CallFunction|Move AxisValue))

(fn ConstructionScript)

(fn CameraTransform
  (Transformation|SetRelativeLocationAndRotation (Variables|Default|GetCamera) (Math|Vector|MakeVector 0.0 0.0 (- (.z (.DevicePosition (Class|HeadMountedDisplayFunctionLibrary|GetOrientationandPosition))) (Variables|/Script/Engine.CapsuleComponent|GetCapsuleHalfHeight (Variables|Collision|GetCapsuleComponent)))) (Math|Rotator|MakeRotator 0.0 0.0 0.0) false false))

(fn CapsuleTransform
  (bind _deviceposition (Class|HeadMountedDisplayFunctionLibrary|GetOrientationandPosition))
  (bind (_devicerotation _deviceposition_2) (Class|HeadMountedDisplayFunctionLibrary|GetOrientationandPosition))
  (Transformation|AddActorLocalOffset (Math|Vector|MakeVector (- (.x _deviceposition) (.x (Variables|Default|GetstoredLocation))) (- (.y _deviceposition) (.y (Variables|Default|GetstoredLocation))) 0.0) false false)
  (Variables|Default|SetstoredLocation (Math|Vector|MakeVector (.x _deviceposition) (.y _deviceposition) 0.0))
  (Transformation|SetActorRotation (Math|Rotator|MakeRotator 0.0 0.0 (.yaw _devicerotation)))
  (Components|Capsule|SetCapsuleHalfHeight (Variables|Collision|GetCapsuleComponent) (/ (.z _deviceposition_2) 2.0) true))

(fn HandOffset
  (bind _deviceposition (Class|HeadMountedDisplayFunctionLibrary|GetOrientationandPosition))
  (Transformation|SetWorldLocationAndRotation (Variables|Default|GetVROrigin) (- (Transformation|GetActorLocation) (Math|Vector|MakeVector (.x _deviceposition) (.y _deviceposition) (Variables|/Script/Engine.CapsuleComponent|GetCapsuleHalfHeight (Variables|Collision|GetCapsuleComponent)))) (Math|Rotator|MakeRotator 0.0 0.0 (- (.yaw (Transformation|GetActorRotation)) (.yaw (.DeviceRotation (Class|HeadMountedDisplayFunctionLibrary|GetOrientationandPosition))))) false false))

(fn Move
  (params (Direction :type Float%20%28single-precision%29))
  (bind _camera (Variables|Default|GetCamera))
  (bind _returnvalue (Math|Vector|GetForwardVector _camera))
  (Pawn|Input|AddMovementInput (Math|Vector|MakeVector (.x _returnvalue) (.y _returnvalue) 0.0) (* (Variables|Default|GetMovementSpeed) Direction) false))

(fn EventGrab)